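; BP_Green is an actor that scatters scenery (a rock, two trees and two bushes) along its local Y axis.
; The GrassSet event moves props to random Y offsets in consecutive bands at a fixed lowered Z, then makes all five visible.
; Bush1 is positioned twice, so its second band wins and Bush is never moved.
; Nothing in this Blueprint calls GrassSet.
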(event `GrassSet`
  (`SceneComponent.K2_SetRelativeLocation` (`self.Rock`) (`KismetMathLibrary.MakeVector` 0.0 (`KismetMathLibrary.RandomFloatInRange` 0.0 708.0) -30.0) false false)
  (`SceneComponent.K2_SetRelativeLocation` (`self.Tree1`) (`KismetMathLibrary.MakeVector` 0.0 (`KismetMathLibrary.RandomFloatInRange` 708.0 1416.0) -30.0) false false)
  (`SceneComponent.K2_SetRelativeLocation` (`self.Bush1`) (`KismetMathLibrary.MakeVector` 0.0 (`KismetMathLibrary.RandomFloatInRange` 1416.0 2196.0) -30.0) false false)
  (`SceneComponent.K2_SetRelativeLocation` (`self.Bush1`) (`KismetMathLibrary.MakeVector` 0.0 (`KismetMathLibrary.RandomFloatInRange` 2196.0 2904.0) -30.0) false false)
  (`SceneComponent.K2_SetRelativeLocation` (`self.Tree`) (`KismetMathLibrary.MakeVector` 0.0 (`KismetMathLibrary.RandomFloatInRange` 2904.0 3612.0) -30.0) false false)
  (`SceneComponent.SetVisibility` (`self.Tree`) true false)
  (`SceneComponent.SetVisibility` (`self.Rock`) true false)
  (`SceneComponent.SetVisibility` (`self.Tree1`) true false)
  (`SceneComponent.SetVisibility` (`self.Bush`) true false)
  (`SceneComponent.SetVisibility` (`self.Bush1`) true false))

(fn `UserConstructionScript`)