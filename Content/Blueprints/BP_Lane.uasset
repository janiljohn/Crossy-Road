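; BP_Lane is one terrain strip (grass, road, river or railroad) in an endless chicken-crossing game.
; InitializeLanes reads the lane type from LaneSpawner, sets the mesh, spawns the matching greenery, water or moving-vehicle actor, then advances the spawner's run countdown.
; When a chicken overlaps its active trigger, it requests a new lane and culls the oldest beyond the limit.
; EndPlay destroys its spawned content.
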(event `self.TriggerZone.OnComponentBeginOverlap`
  (params (OverlappedComponent :type "PrimitiveComponent Object Reference") (OtherActor :type "Actor Object Reference") (OtherComp :type "PrimitiveComponent Object Reference") (OtherBodyIndex :type Integer) (bFromSweep :type Boolean) (SweepResult :type "HitResult Structure (by ref)"))
  (bind _lanespawner (`self.LaneSpawner`))
  (bind _lanespawner_2 (`self.LaneSpawner`))
  (bind _lanearray (`/Game/Blueprints/BP_LaneSpawner.laneArray` _lanespawner_2))
  (if (`self.triggerActive`)
    (cast `/Game/Blueprints/BP_Chicken` OtherActor)
    (`/Game/Blueprints/BP_LaneSpawner.Spawn Lane at Spawn Point` _lanespawner)
    (if (> (`/Game/Blueprints/BP_LaneSpawner.lane_count` _lanespawner) (`/Game/Blueprints/BP_LaneSpawner.lane_max` _lanespawner))
      (`self.K2_DestroyActor` (`|GetArrayItem` _lanearray))
      (`KismetArrayLibrary.Array_Remove` _lanearray)
      (bind _result (`/Engine/EditorBlueprintResources/StandardMacros.DecrementInt` (`/Game/Blueprints/BP_LaneSpawner.lane_count` _lanespawner_2))
        (:`  `
          (set `/Game/Blueprints/BP_LaneSpawner.lane_count` _result _lanespawner_2))))))

(event `self.ReceiveEndPlay`
  (params (EndPlayReason :type "EEndPlayReason Enum" :default "Destroyed"))
  (`/Engine/EditorBlueprintResources/StandardMacros.IsValid` (`self.curGrass`)
    (:`Is Valid`
      (`self.K2_DestroyActor` (`self.curGrass`)))
    (:`Is Not Valid`
      _))
  (`/Engine/EditorBlueprintResources/StandardMacros.IsValid` (`self.curVehicle`)
    (:`Is Valid`
      (`self.K2_DestroyActor` (`self.curVehicle`)))
    (:`Is Not Valid`
      _))
  (`/Engine/EditorBlueprintResources/StandardMacros.IsValid` (`self.curRiver`)
    (:`Is Valid`
      (`self.K2_DestroyActor` (`self.curRiver`)))))

(fn `initializeLanes`
  (switch `int` (`/Game/Blueprints/BP_LaneSpawner.laneMesh` (`self.LaneSpawner`))
    (:`0`
      (`self.prepareGrass`))
    (:`1`
      (`self.prepareRoad`))
    (:`2`
      (`self.prepareRiver`))
    (:`3`
      (`self.prepareRailroad`)))
  (`self.updateVariables`))

(fn `prepareGrass`
  (`SceneComponent.K2_AddLocalOffset` (`self.LaneMesh`) (0.0 0.0 -12.0) false false)
  (if (== (`/Game/Blueprints/BP_LaneSpawner.laneMeshCount` (`self.LaneSpawner`)) 2)
    (set `/Game/Blueprints/BP_LaneSpawner.grassRemaining` (`KismetMathLibrary.RandomInteger` 2) (`self.LaneSpawner`)))
  (if (== (`/Game/Blueprints/BP_LaneSpawner.grassRemaining` (`self.LaneSpawner`)) 0)
    (`StaticMeshComponent.SetStaticMesh` (`self.LaneMesh`) "/Game/Lanes/LightGrass.LightGrass")
    (else
      (`StaticMeshComponent.SetStaticMesh` (`self.LaneMesh`) "/Game/Lanes/DarkGrass.DarkGrass")))
  (bind _returnvalue (`|SpawnActorFromClass` "/Game/Blueprints/BP_Green.BP_Green_C" (`KismetMathLibrary.Conv_VectorToTransform` (`SceneComponent.K2_GetComponentLocation` (`self.VehicleSpawn`))) "Undefined" "OverrideRootScale" null null))
  (bind _output_get (set `self.curGrass` _returnvalue))
  (`/Game/Blueprints/BP_Green.GrassSet` _output_get))

(fn `prepareRailroad`
  (`SceneComponent.K2_AddLocalOffset` (`self.LaneMesh`) (0.0 0.0 -18.75) false false)
  (`StaticMeshComponent.SetStaticMesh` (`self.LaneMesh`) "/Game/Lanes/RailroadFixed.RailroadFixed")
  (`self.Spawn Moving Vehicle`)
  (`/Game/Blueprints/BP_MovingVehicle.TrainLane` (`self.curVehicle`)))

(fn `prepareRiver`
  (`StaticMeshComponent.SetStaticMesh` (`self.LaneMesh`) "/Game/Lanes/River.River")
  (bind _returnvalue (`|SpawnActorFromClass` "/Game/Blueprints/BP_Water.BP_Water_C" (`KismetMathLibrary.Conv_VectorToTransform` (`SceneComponent.K2_GetComponentLocation` (`self.VehicleSpawn`))) "Undefined" "OverrideRootScale" null null))
  (bind _output_get (set `self.curRiver` _returnvalue))
  (`/Game/Blueprints/BP_Water.RiverSet` _output_get))

(fn `prepareRoad`
  (if (== (`/Game/Blueprints/BP_LaneSpawner.laneMeshCount` (`self.LaneSpawner`)) 4)
    (`StaticMeshComponent.SetStaticMesh` (`self.LaneMesh`) "/Game/Lanes/UnmarkedRoad.UnmarkedRoad")
    (else
      (`StaticMeshComponent.SetStaticMesh` (`self.LaneMesh`) "/Game/Lanes/MarkedRoad.MarkedRoad")))
  (`self.Spawn Moving Vehicle`)
  (`/Game/Blueprints/BP_MovingVehicle.RoadLane` (`self.curVehicle`)))

(fn `Spawn Moving Vehicle`
  (bind _returnvalue (`|SpawnActorFromClass` "/Game/Blueprints/BP_MovingVehicle.BP_MovingVehicle_C" (`KismetMathLibrary.Conv_VectorToTransform` (`SceneComponent.K2_GetComponentLocation` (`self.VehicleSpawn`))) "Undefined" "OverrideRootScale" null null))
  (set `self.curVehicle` _returnvalue)
  (set `/Game/Blueprints/BP_MovingVehicle.ParentLane` self (`self.curVehicle`)))

(fn `updateVariables`
  (`/Engine/EditorBlueprintResources/StandardMacros.DecrementInt` (`/Game/Blueprints/BP_LaneSpawner.laneMeshCount` (`self.LaneSpawner`))
    (:`  `
      (if (<= (`/Game/Blueprints/BP_LaneSpawner.laneMeshCount` (`self.LaneSpawner`)) 0)
        (`/Game/Blueprints/BP_LaneSpawner.prepareLaneValues` (`self.LaneSpawner`))))))

(fn `UserConstructionScript`)