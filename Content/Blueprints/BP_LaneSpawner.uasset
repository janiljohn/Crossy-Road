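; Spawner that builds the chain of BP_Lane segments, clearing existing lanes and seeding five from the player's position at start and restart.
; Each lane spawns at the previous one's SpawnPoint, receives a spawner reference and initializes itself.
; Once LaneCount reaches LaneMax, triggers on older lanes are switched off.
; PrepareLaneValues randomly picks a mesh type differing from the last, with a fixed count per type.
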(event `self.ReceiveBeginPlay`
  (`self.SpawnInitialLanes`))

(fn `prepareLane`
  (if (== (`self.laneMesh`) -1)
    (set `self.laneMesh` 0)
    (set `self.laneMeshCount` 2))
  (`/Game/Blueprints/BP_Lane.initializeLanes` (`self.NewestLane`)))

(fn `prepareLaneValues`
  (bind _output_get (set `self.meshRemaining` (select `int` (`KismetMathLibrary.RandomInteger` 4) :`0` 0 :`1` 1 :`2` 2 :`3` 3)))
  (if (== _output_get (`self.laneMesh`))
    (bind _result (`/Engine/EditorBlueprintResources/StandardMacros.DecrementInt` (`self.meshRemaining`))
      (:`  `
        (set `self.meshRemaining` (`KismetMathLibrary.Abs_Int` _result)))))
  (set `self.laneMesh` (`self.meshRemaining`))
  (set `self.laneMeshCount` (select `int` (`self.laneMesh`) :`0` 4 :`1` 3 :`2` 6 :`3` 2)))

(fn `prepareTriggers`
  (bind _lanearray (`self.laneArray`))
  (bind _lanearray_2 (`self.laneArray`))
  (if (> (`self.lane_max`) (`self.lane_count`))
    _
    (elif (`self.startTrigger`)
      (set `/Game/Blueprints/BP_Lane.triggerActive` false (`|GetArrayItem` _lanearray (- (/ (`KismetArrayLibrary.Array_Length` _lanearray) 2) 1)))
      (else
        (for (_array_element _array_index) _lanearray_2
          (if (< _array_index (/ (`KismetArrayLibrary.Array_Length` _lanearray_2) 2))
            (set `/Game/Blueprints/BP_Lane.triggerActive` false _array_element)
            (set `self.startTrigger` true)))))))

(fn `restartGame`
  (`GameModeBase.RestartPlayer` (`GameplayStatics.GetGameMode`) null)
  (set `self.lane_count` 0)
  (set `self.laneMesh` 0)
  (set `self.laneMeshCount` 2)
  (set `self.NewestLane` null)
  (`KismetArrayLibrary.Array_Clear` (`self.laneArray`))
  (`self.SpawnInitialLanes`))

(fn `Spawn Lane at Spawn Point`
  (`self.SpawnLane` (`SceneComponent.K2_GetComponentLocation` (`/Game/Blueprints/BP_Lane.SpawnPoint` (`self.NewestLane`)))))

(fn `SpawnInitialLanes`
  (`|ExecutionSequence`
    (:`then_0`
      (bind _outactors (`GameplayStatics.GetAllActorsOfClass` "/Game/Blueprints/BP_Lane.BP_Lane_C"))
      (for _array_element _outactors
        (`self.K2_DestroyActor` _array_element)))
    (:`then_1`
      (for _ (range 5)
        (`/Engine/EditorBlueprintResources/StandardMacros.IsValid` (`self.NewestLane`)
          (:`Is Valid`
            (`self.Spawn Lane at Spawn Point`))
          (:`Is Not Valid`
            (`self.SpawnLane` (`self.K2_GetActorLocation` (`GameplayStatics.GetPlayerPawn` 0)))))))))

(fn `SpawnLane`
  (params (`Spawn Location` :type "Vector Structure"))
  (`self.prepareTriggers`)
  (bind _result (`/Engine/EditorBlueprintResources/StandardMacros.IncrementInt` (`self.lane_count`))
    (:`  `
      (set `self.lane_count` _result)
      (bind _returnvalue (`|SpawnActorFromClass` "/Game/Blueprints/BP_Lane.BP_Lane_C" (`KismetMathLibrary.MakeTransform` (`KismetMathLibrary.MakeVector` (+ `Spawn Location_X` 40.0) (`self.ycoord`) (`self.zcoord`))) "Undefined" "OverrideRootScale" null null))
      (bind _output_get (set `self.NewestLane` _returnvalue))
      (`KismetArrayLibrary.Array_Add` (`self.laneArray`) (`self.NewestLane`))
      (set `/Game/Blueprints/BP_Lane.LaneSpawner` self _output_get)
      (`self.prepareLane`))))

(fn `UserConstructionScript`)