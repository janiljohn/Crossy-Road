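; Moving hazard actor for road and train lanes that restarts the game through its lane spawner on overlapping BP_Chicken.
; RoadLane picks a random vehicle mesh, enables an animated police light for one variant, then uses a timeline to drive it along Y in a random direction, looping after random delays.
; TrainLane shows train meshes after a random delay, stretches the collision box and moves along Y by timeline.
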(event `RoadLane`
  (`self.prepRoadMesh`)
  (`SceneComponent.SetVisibility` (`self.VehicleMesh`) false false :!label _label)
  (`KismetSystemLibrary.Delay` (`KismetMathLibrary.RandomFloatInRange` 0.0 3.0))
  (`SceneComponent.SetVisibility` (`self.VehicleMesh`) true false)
  (if (== (`KismetMathLibrary.RandomInteger` 2) 0)
    (`self.K2_SetActorRotation` (struct))
    (bind (_direction _position) (`Timeline|Road Movement` :!via `PlayFromStart` :!label _label_2)
      (:`Update`
        (`self.K2_SetActorLocation` (`KismetMathLibrary.MakeVector` (`self.originalX`) (.y _position))))
      (:`Finished`
        (`self.K2_SetActorLocation` (`KismetMathLibrary.MakeVector` (`self.originalX`) -1770.0))
        (goto _label)))
    (else
      (`self.K2_SetActorRotation` (struct :`Yaw` 180.0))
      (goto _label_2 :!via `ReverseFromEnd`))))

(event `TrainLane`
  (`KismetSystemLibrary.Delay` (`KismetMathLibrary.RandomFloatInRange` 0.0 3.0))
  (`SceneComponent.SetVisibility` (`self.TrainF`) true false)
  (`SceneComponent.SetVisibility` (`self.TrainC1`) true false)
  (`SceneComponent.SetVisibility` (`self.TrainC2`) true false)
  (`SceneComponent.SetVisibility` (`self.TrainC3`) true false)
  (`SceneComponent.K2_SetRelativeLocation` (`self.collisionBox`) (5.0 500.0 30.0) false false)
  (`SceneComponent.SetRelativeScale3D` (`self.collisionBox`) (1.0 31.0 1.0))
  (bind (_direction _position) (`Timeline|Train Movement`)
    (:`Update`
      (`self.K2_SetActorLocation` (`KismetMathLibrary.MakeVector` (`self.originalX`) (.y _position))))))

(event `self.collisionBox.OnComponentBeginOverlap`
  (params (OverlappedComponent :type "PrimitiveComponent Object Reference") (OtherActor :type "Actor Object Reference") (OtherComp :type "PrimitiveComponent Object Reference") (OtherBodyIndex :type Integer) (bFromSweep :type Boolean) (SweepResult :type "HitResult Structure (by ref)"))
  (cast `/Game/Blueprints/BP_Chicken` OtherActor)
  (`/Game/Blueprints/BP_LaneSpawner.restartGame` (`/Game/Blueprints/BP_Lane.LaneSpawner` (`self.ParentLane`))))

(event `self.ReceiveBeginPlay`
  (bind _returnvalue_x (`KismetMathLibrary.BreakVector` (`self.K2_GetActorLocation`)))
  (set `self.originalX` _returnvalue_x))

(event `PoliceCarLight`
  (bind (_direction _blue_track) (`Timeline|Timeline`)
    (:`Update`
      (`LightComponent.SetLightColor` (`self.blue`) _blue_track true))))

(fn `prepRoadMesh`
  (`StaticMeshComponent.SetStaticMesh` (`self.VehicleMesh`) (select `int` (`KismetMathLibrary.RandomInteger` 9) :`0` "/Game/Vehicles/FedExTruck.FedExTruck" :`1` "/Game/Vehicles/hummer.hummer" :`2` "/Game/Vehicles/long_car_Rolls_Royce.long_car_Rolls_Royce" :`3` "/Game/Vehicles/policeCar_policeCar.policeCar_policeCar" :`4` "/Game/Vehicles/suv_Untitled.suv_Untitled" :`5` "/Game/Vehicles/taxi_taxi.taxi_taxi" :`6` "/Game/Vehicles/uspsTruck.uspsTruck" :`7` "/Game/Vehicles/pizza_car.pizza_car" :`8` "/Game/Vehicles/upsTruck.upsTruck" :!type "StaticMesh Object Reference"))
  (if (== (`self.VehicleMesh`) null)
    (`SceneComponent.SetVisibility` (`self.blue`) true false)
    (`self.PoliceCarLight`)
    (else
      (`SceneComponent.SetVisibility` (`self.blue`) false false))))

(fn `UserConstructionScript`)