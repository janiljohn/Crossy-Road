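; BP_Water is a river actor with five platforms that move with it along the Y axis.
; A RiverSet event waits a random delay of up to three seconds, makes the platforms visible, then plays a timeline.
; Each timeline update sets the actor location using the animated Y and the X cached at BeginPlay, leaving Z unwired.
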(event `RiverSet`
  (`KismetSystemLibrary.Delay` (`KismetMathLibrary.RandomFloatInRange` 0.0 3.0))
  (`SceneComponent.SetVisibility` (`self.platform1`) true false)
  (`SceneComponent.SetVisibility` (`self.platform2`) true false)
  (`SceneComponent.SetVisibility` (`self.platform3`) true false)
  (`SceneComponent.SetVisibility` (`self.platform4`) true false)
  (`SceneComponent.SetVisibility` (`self.platform5`) true false)
  (bind (_direction _position) (`Timeline|Timeline`)
    (:`Update`
      (`self.K2_SetActorLocation` (`KismetMathLibrary.MakeVector` (`self.ogX`) (.y _position))))))

(event `self.ReceiveBeginPlay`
  (bind _returnvalue_x (`KismetMathLibrary.BreakVector` (`self.K2_GetActorLocation`)))
  (set `self.ogX` _returnvalue_x))

(fn `UserConstructionScript`)